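; TestEnemyAIController is the AI controller for a test enemy in the SpaceShoot game.
; On possess, it sets up TestEnemyBlackboard and derives two points from the pawn's starting location.
; Position1 lies below that location and Position2 is offset from Position1 along world X.
; It then runs TestEnemyBehaviourTree, with both points available to it as blackboard vectors.
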(event EventOnPossess
  (params (PossessedPawn :type Pawn%20Object%20Reference))
  (bind _self self)
  (bind _returnvalue (AI|GetBlackboard _self))
  (bind _returnvalue_2 (Pawn|GetControlledPawn _self))
  (bind _returnvalue_3 (Transformation|GetActorLocation _returnvalue_2))
  (bind _returnvalue_4 (+ _returnvalue_3 "0,0.000000,-300.000000"))
  (Class|AIController|UseBlackboard "/Game/SpaceShoot/Blueprint/BehaviourTree/TestEnemyBlackboard.TestEnemyBlackboard")
  (AI|Components|Blackboard|SetValueasVector _returnvalue (Variables|Default|GetPosition1) _returnvalue_4)
  (AI|Components|Blackboard|SetValueasVector _returnvalue (Variables|Default|GetPosition2) (+ _returnvalue_4 "300.000000, 0, 0"))
  (AI|RunBehaviorTree "/Game/SpaceShoot/Blueprint/BehaviourTree/TestEnemyBehaviourTree.TestEnemyBehaviourTree"))

(fn ConstructionScript)